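; AI director component that runs bot races toward a target, with setup done on the server.
; On BeginPlay it names every AI_Base bot and binds catch and game-end events.
; While the game runs, StartRace compares navmesh path lengths, holding the farthest bot and sending the others to the target.
; A catch halts all bots, flags winners by highest points and ends the GameState round; match end also halts them.
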(event `self.ReceiveBeginPlay`
  (`/Engine/EditorBlueprintResources/ActorComponentMacros.Switch Has Authority`
    (:`Authority`
      (`|ExecutionSequence`
        (:`then_0`
          (bind _assa_game_state (cast `/Game/_Gameplay/_Common/SA_GameState` (`GameplayStatics.GetGameState`)))
          (bind _output_get (set `self.@GameState` _assa_game_state))
          (add `/Game/_Gameplay/_Common/SA_GameState.cbGameEnded` _output_get (`|CreateDelegate` :!event `onMatchEnd`)))
        (:`then_1`
          (bind _outactors (`GameplayStatics.GetAllActorsOfClass` "/Game/_Gameplay/AI/AI_Base.AI_Base_C"))
          (bind _output_get_2 (set `self.@AI's` _outactors))
          (add `/Game/_Gameplay/AI/AI_Base.cbCatch` _output_get_2 (`|CreateDelegate` :!event `onAnyAICatch`))
          (for (_array_element _array_index) (`self.@AI's`)
            (`/Game/_Gameplay/AI/AI_Base.!SetName(ToServer)` _array_element (`KismetStringLibrary.Concat_StrStr` "Bot_" (`KismetStringLibrary.Conv_IntToString` (+ _array_index 1))))))))))

(event `!StartRace`
  (params (Target :type "Actor Object Reference"))
  (if (`self.!AllowRace`)
    (`self.!MoveAIToTarget` Target)))

(fn `!AllowRace`
  (returns (Result :type Boolean))
  (bind __gamestate (`self.@GameState`)
    (:`then`
      (return (`/Game/_Gameplay/_Common/SA_GameState.!IsGameStarted` __gamestate)))
    (:`else`
      (return false))))

(fn `!MoveAIToTarget`
  (params (`#Target` :type "Actor Object Reference"))
  (locals (`#PathLength's` :type "Array of Float (double-precision)"))
  (bind __ai_s (`self.@AI's`))
  (if (> (`KismetArrayLibrary.Array_Length` (`self.@AI's`)) 1)
    (for (_array_element _array_index) (`self.@AI's`)
      (bind _returnvalue (`NavigationSystemV1.FindPathToLocationSynchronously` (`Actor.K2_GetActorLocation` _array_element) (`Actor.K2_GetActorLocation` (`local.#Target`)) null "/Script/NavigationSystem.RecastFilter_UseDefaultArea"))
      (`KismetArrayLibrary.Array_Set` (`local.#PathLength's`) _array_index (`NavigationPath.GetPathLength` _returnvalue) true))
    (for (_array_element_2 _array_index_2) (`self.@AI's`)
      (if (== _array_index_2 (`KismetMathLibrary.MaxOfFloatArray` (`local.#PathLength's`)))
        (`/Game/_Gameplay/AI/AI_Base.!Stay(ToServer)` _array_element_2)
        (else
          (`/Game/_Gameplay/AI/AI_Base.!MoveToTarget(ToServer)` _array_element_2 (`local.#Target`)))))
    (elif (`KismetArrayLibrary.Array_IsValidIndex` __ai_s)
      (`/Game/_Gameplay/AI/AI_Base.!MoveToTarget(ToServer)` (`|GetArrayItem` __ai_s) (`local.#Target`)))))

(fn `onAnyAICatch`
  (locals (`#Points` :type "Array of Integer"))
  (`|ExecutionSequence`
    (:`then_0`
      (for _array_element (`self.@AI's`)
        (`/Game/_Gameplay/AI/AI_Base.!Stay(ToServer)` _array_element)
        (`KismetArrayLibrary.Array_Add` (`local.#Points`) (`/Game/_Gameplay/AI/AI_Base.@Points` _array_element)))
      (for _array_element_2 (`self.@AI's`)
        (set `/Game/_Gameplay/AI/AI_Base.@IsWinner` (== (`/Game/_Gameplay/AI/AI_Base.@Points` _array_element_2) (`.MaxValue` (`KismetMathLibrary.MaxOfIntArray` (`local.#Points`)))) _array_element_2)))
    (:`then_1`
      (bind __gamestate (`self.@GameState`)
        (:`then`
          (`/Game/_Gameplay/_Common/SA_GameState.!RoundEnd` __gamestate))
        (:`else`)))))

(fn `onMatchEnd`
  (for _array_element (`self.@AI's`)
    (`/Game/_Gameplay/AI/AI_Base.!Stay(ToServer)` _array_element)))