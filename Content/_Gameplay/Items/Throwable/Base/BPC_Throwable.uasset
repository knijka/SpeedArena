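; Throwable item component that launches its owning actor as a bouncing projectile through a server event.
; Throw detaches the owner, adds a projectile movement component at runtime and passes the owner to the game mode's AI Director to start a race.
; Velocity follows the holder's instigator control rotation, falling back to the holder's forward vector.
; Projectile bounce and stop both fire the Bounced callback.
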(event `!Throw(ToServer)`
  (`self.!Throw`))

(fn `!CalculateVelocity`
  (returns (Velocity :type "Vector Structure"))
  (bind __speed (`self.@Speed`))
  (bind _returnvalue (`Actor.GetOwner` (`self.GetOwner`)))
  (bind _instigator (`Actor.Instigator` _returnvalue))
  (`/Engine/EditorBlueprintResources/StandardMacros.IsValid` _instigator
    (:`Is Valid`
      (return (* (`KismetMathLibrary.Conv_RotatorToVector` (`Pawn.GetControlRotation` _instigator)) (`KismetSystemLibrary.MakeLiteralDouble` __speed))))
    (:`Is Not Valid`
      (return (* (`Actor.GetActorForwardVector` _returnvalue) (`KismetSystemLibrary.MakeLiteralDouble` __speed))))))

(fn `!Throw`
  (bind _returnvalue (`self.GetOwner`))
  (bind __speed (`self.@Speed`))
  (`Actor.K2_DetachFromActor` _returnvalue "KeepWorld" "KeepWorld" "KeepRelative")
  (bind _returnvalue_2 (`|AddComponentByClass` _returnvalue "/Script/Engine.ProjectileMovementComponent"))
  (`|ExecutionSequence`
    (:`then_0`
      (add `ProjectileMovementComponent.OnProjectileBounce` _returnvalue_2 (`|CreateDelegate` :!event `onProjectileBounce`))
      (add `ProjectileMovementComponent.OnProjectileStop` _returnvalue_2 (`|CreateDelegate` :!event `onProjectileStop`)))
    (:`then_1`
      (set `MovementComponent.Velocity` (`self.!CalculateVelocity`) _returnvalue_2)
      (set `ProjectileMovementComponent.InitialSpeed` __speed _returnvalue_2)
      (set `ProjectileMovementComponent.MaxSpeed` __speed _returnvalue_2)
      (set `ProjectileMovementComponent.bShouldBounce` true _returnvalue_2)
      (`/Game/_Gameplay/AI/BPC_AI_Director.!StartRace` (`Actor.GetComponentByClass` (`GameplayStatics.GetGameMode`) "/Game/_Gameplay/AI/BPC_AI_Director.BPC_AI_Director_C") (`self.GetOwner`)))))

(fn `onProjectileBounce`
  (params (ImpactResult :type "HitResult Structure (by ref)") (ImpactVelocity :type "Vector Structure (by ref)"))
  (`self.cbBounced`))

(fn `onProjectileStop`
  (params (ImpactResult :type "HitResult Structure (by ref)"))
  (`self.cbBounced`))